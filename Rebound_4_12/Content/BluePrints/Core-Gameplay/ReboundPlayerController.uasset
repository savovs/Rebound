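; Player controller for Rebound that routes one player's input to their pawn and to UI, using a shared camera actor as its view.
; It forwards move, dash, throw and per-tick aim to the pawn, relays menu buttons through Call events and toggles the pause menu.
; SpawnPawn spawns and possesses the character with a player-coloured beam effect, then applies customisation and game-mode stats.
; It also controls looping charge rumble; indicator and respawn-check logic are unused.
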(event `AddIndicator`
  ;[1 1 1] Deprecated - leave here just incase
  (cast `/Game/BluePrints/Gamemodes/ReboundGameMode` (`GameplayStatics.GetGameMode`))
  (bind _returnvalue (`|CreateWidget` "/Game/UI/InGame/PlayerIndicators.PlayerIndicators_C" self))
  (`UserWidget.AddToViewport` _returnvalue 0)
  (`KismetSystemLibrary.PrintString` "added indicator" (`/Game/BluePrints/data/PersistentData.isDevMode` (`self.persisData`))))

(event `self.ReceiveBeginPlay`
  (bind _aspersistent_data (cast `/Game/BluePrints/data/PersistentData` (`GameplayStatics.GetGameInstance`)))
  (set `self.persisData` _aspersistent_data)
  (bind _outactors (`GameplayStatics.GetAllActorsOfClass` "/Game/BluePrints/Core-Gameplay/SharedCameraActor.SharedCameraActor_C"))
  (if (> (`KismetArrayLibrary.Array_Length` _outactors) 0)
    (`self.SetViewTargetWithBlend` (`KismetArrayLibrary.Array_Get` _outactors))))

(event `self.ReceiveTick`
  (params (DeltaSeconds :type "Float (single-precision)"))
  (`self.SetAimVector`))

(event `InputAction|Confirm` :paused true
  (params (Key :type "Key Structure" :default "AnyKey"))
  ;[1 1 1] UI InputEvents
  (:`Pressed`
    (`self.ButtonConfirm`)))

(event `InputAction|swapUIRight` :paused true
  (params (Key :type "Key Structure" :default "AnyKey"))
  ;[1 1 1] UI InputEvents
  (:`Pressed`
    (`self.ButtonRight`)))

(event `InputAction|swapUIleft` :paused true
  (params (Key :type "Key Structure" :default "AnyKey"))
  ;[1 1 1] UI InputEvents
  (:`Pressed`
    (`self.ButtonLeft`)))

(event `InputAction|DownUI` :paused true
  (params (Key :type "Key Structure" :default "AnyKey"))
  ;[1 1 1] UI InputEvents
  (:`Pressed`
    (`self.ButtonDown`)))

(event `InputAction|UpUI` :paused true
  (params (Key :type "Key Structure" :default "AnyKey"))
  ;[1 1 1] UI InputEvents
  (:`Pressed`
    (`self.ButtonUp`)))

(event `InputAction|Escape` :paused true
  (params (Key :type "Key Structure" :default "AnyKey"))
  (bind _pausemenureference (`self.PauseMenuReference`))
  (bind _pausemenureference_2 (`self.PauseMenuReference`))
  ;[0 0.1276 1] Start Button Pressed
  ;;[1 1 1] UI InputEvents
  (:`Pressed`
    (`self.ButtonEscape`)
    (bind _returnvalue (`GameplayStatics.GetCurrentLevelName` true))
    (if (and (`KismetStringLibrary.NotEqual_StrStr` _returnvalue "MainMenu") (not (`GameplayStatics.IsGamePaused`)))
      (`/Engine/EditorBlueprintResources/StandardMacros.IsValid` _pausemenureference
        (:`Is Valid`
          _)
        (:`Is Not Valid`
          (bind _returnvalue_2 (`|CreateWidget` "/Game/UI/InGame/InGamePause.InGamePause_C" self))
          (set `self.PauseMenuReference` _returnvalue_2)))
      (`/Game/UI/InGame/InGamePause.SetOwnerEvent` _pausemenureference_2)
      (`UserWidget.AddToViewport` _pausemenureference_2 0)
      (`GameplayStatics.SetGamePaused` true)
      (`WidgetBlueprintLibrary.SetInputMode_UIOnlyEx` null _pausemenureference_2)
      (else
        (if (!= _pausemenureference null) :!label _label
          (if (`Widget.IsInViewport` _pausemenureference)
            (`GameplayStatics.SetGamePaused` false)
            (`Widget.RemoveFromParent` _pausemenureference)
            (`WidgetBlueprintLibrary.SetInputMode_GameOnly` null)))))))

(event `InputAction|Exit` :paused true
  (params (Key :type "Key Structure" :default "AnyKey"))
  ;[0 0.1276 1] Start Button Pressed
  ;;[1 1 1] UI InputEvents
  (:`Pressed`
    (`self.ButtonBack`)
    (if (`GameplayStatics.IsGamePaused`)
      (goto _label))))

(event `PlayChargeEffect`
  (`/Engine/EditorBlueprintResources/StandardMacros.DoOnce` false :!label _label_2
    (:`Completed`
      (`self.ClientPlayForceFeedback` "/Game/BluePrints/Core-Gameplay/Characters/Charge.Charge" true)
      (goto _label_3 :!via `Reset`))))

(event `StopChargeEffect`
  (`/Engine/EditorBlueprintResources/StandardMacros.DoOnce` true :!label _label_3
    (:`Completed`
      (`self.ClientStopForceFeedback` "/Game/BluePrints/Core-Gameplay/Characters/Charge.Charge")
      (goto _label_2 :!via `Reset`))))

(event `stopallfeedback`
  (`self.ClientStopForceFeedback` "/Game/BluePrints/Core-Gameplay/Characters/Charge.Charge"))

(event `InputAction|Dash`
  (params (Key :type "Key Structure" :default "AnyKey"))
  (bind _playerpawn (`self.PlayerPawn`))
  (:`Pressed`
    (`/Engine/EditorBlueprintResources/StandardMacros.IsValid` _playerpawn
      (:`Is Valid`
        (`/Game/BluePrints/Core-Gameplay/Characters/ReboundPlayerCharacter.DashEvent` _playerpawn)))))

(event `InputAction|PickUp`
  (params (Key :type "Key Structure" :default "AnyKey"))
  (bind _playerpawn (`self.PlayerPawn`))
  (:`Pressed`
    (`/Engine/EditorBlueprintResources/StandardMacros.IsValid` _playerpawn
      (:`Is Valid`
        (`/Game/BluePrints/Core-Gameplay/Characters/ReboundPlayerCharacter.ThrowEventStart` _playerpawn))))
  (:`Released`
    (`/Engine/EditorBlueprintResources/StandardMacros.IsValid` _playerpawn
      (:`Is Valid`
        (`/Game/BluePrints/Core-Gameplay/Characters/ReboundPlayerCharacter.ThrowEventRelease` _playerpawn)))))

(event `InputAxis|Vertical`
  (params (AxisValue :type "Float (single-precision)"))
  (bind _playerpawn (`self.PlayerPawn`))
  (`/Engine/EditorBlueprintResources/StandardMacros.IsValid` _playerpawn
    (:`Is Valid`
      (`/Game/BluePrints/Core-Gameplay/Characters/ReboundPlayerCharacter.MoveVertical` _playerpawn AxisValue))))

(event `InputAxis|Horizontal`
  (params (AxisValue :type "Float (single-precision)"))
  (bind _playerpawn (`self.PlayerPawn`))
  (`/Engine/EditorBlueprintResources/StandardMacros.IsValid` _playerpawn
    (:`Is Valid`
      (`/Game/BluePrints/Core-Gameplay/Characters/ReboundPlayerCharacter.MoveHorizontal` _playerpawn AxisValue))))

(fn `RespawnCheck`
  ;[1 1 1] Unused
  (if (`self.CanRespawn`)
    (if (== (`self.K2_GetPawn`) null)
      (bind _output_get (set `self.RespawnTimerCur` (+ (`self.RespawnTimerCur`) (`GameplayStatics.GetWorldDeltaSeconds`))))
      (if (>= _output_get (`self.RespawnTimerMax`))
        (set `self.RespawnTimerCur` (`self.RespawnTimerMax`))
        (cast `/Game/BluePrints/Gamemodes/ReboundGameMode` (`GameplayStatics.GetGameMode`))))))

(fn `SetAimVector`
  (bind _playerpawn (`self.PlayerPawn`))
  (`/Engine/EditorBlueprintResources/StandardMacros.IsValid` _playerpawn
    (:`Is Valid`
      (set `/Game/BluePrints/Core-Gameplay/Characters/ReboundPlayerCharacter.AimVector` (`KismetMathLibrary.MakeVector2D` (`self.GetInputAxisValue`) (`self.GetInputAxisValue`)) _playerpawn))))

(fn `SpawnPawn`
  (params (SpawnPoint :type "Transform Structure") (playerPawn :type "/Game/BluePrints/Core-Gameplay/Characters/ReboundPlayerCharacter Class Reference"))
  (bind _location (.location SpawnPoint))
  (bind _item_charcolour (break `/Game/BluePrints/Core-Gameplay/Characters/CustomCharacterStats` (`KismetArrayLibrary.Array_Get` (`/Game/BluePrints/data/PersistentData.PlayerCharacters` (`self.persisData`)) (`self.PlayerID`))))
  (if (== (`self.K2_GetPawn`) null)
    (bind _returnvalue (`GameplayStatics.SpawnEmitterAtLocation` "/Game/Art/Particles/Spawn_Beam.Spawn_Beam" _location (.rotation SpawnPoint)))
    (`ParticleSystemComponent.SetBeamSourcePoint` _returnvalue 0 _location 0)
    (`ParticleSystemComponent.SetBeamTargetPoint` _returnvalue 0 (`KismetMathLibrary.MakeVector` (.x _location) (.y _location) 8000.0) 0)
    (`ParticleSystemComponent.SetColorParameter` _returnvalue "InstancedParticleColor" _item_charcolour)
    (bind _returnvalue_2 (`|SpawnActorFromClass` playerPawn SpawnPoint "Undefined" "OverrideRootScale"))
    (`self.Possess` _returnvalue_2)
    (`/Game/BluePrints/Core-Gameplay/Characters/ReboundPlayerCharacter.SetTokenColour` _returnvalue_2)
    (`KismetSystemLibrary.PrintString` (`KismetStringLibrary.Conv_IntToString` (`self.PlayerID`)) (`/Game/BluePrints/data/PersistentData.isDevMode` (`self.persisData`)) true (struct :`A` 1.0) 10.0)
    (`/Game/BluePrints/Core-Gameplay/Characters/ReboundPlayerCharacter.setCustomCharacter` _returnvalue_2)
    (bind _asrebound_game_mode (cast `/Game/BluePrints/Gamemodes/ReboundGameMode` (`GameplayStatics.GetGameMode`)))
    (`/Game/BluePrints/Core-Gameplay/Characters/ReboundPlayerCharacter.SetUpStats` _returnvalue_2 (`/Game/BluePrints/data/GameData.PlayerVariantName` (`/Game/BluePrints/Gamemodes/ReboundGameMode.gameData` _asrebound_game_mode)))
    (set `self.PlayerPawn` _returnvalue_2)))

(fn `UserConstructionScript`)