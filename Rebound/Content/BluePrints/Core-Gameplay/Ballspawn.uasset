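; Ball spawn point actor that records its spawn location and tracks whether that spot is blocked.
; On BeginPlay it stores the SpawnPosition world location and caches the PersistentData game instance.
; Every Tick, a small sphere overlap on pawns and one other object type updates IsObstructed and ObstructionActors; no spawning happens here.
; A dev-mode debug sphere colored by obstruction state is present but disconnected.
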(event `self.ReceiveBeginPlay`
  (set `self.SpawnLocation` (`SceneComponent.K2_GetComponentLocation` (`self.SpawnPosition`)))
  (bind _aspersistent_data (cast `/Game/BluePrints/data/PersistentData` (`GameplayStatics.GetGameInstance`)))
  (set `self.persisData` _aspersistent_data))

(event `self.ReceiveTick`
  (params (DeltaSeconds :type "Float (single-precision)"))
  (bind (_outactors _returnvalue) (`KismetSystemLibrary.SphereOverlapActors_NEW` (`SceneComponent.K2_GetComponentLocation` (`self.SpawnPosition`)) 30.0 (`|MakeArray` "ObjectTypeQuery3" "ObjectTypeQuery7" :!type "EObjectTypeQuery Enum") "/Script/Engine.Actor"))
  (set `self.ObstructionActors` _outactors)
  (bind _output_get (set `self.IsObstructed` _returnvalue)))

(fn `UserConstructionScript`)