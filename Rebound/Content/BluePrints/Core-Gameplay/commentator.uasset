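; Match commentator for Rebound that prints random lines reacting to game events, currently as on-screen text.
; On BeginPlay it binds to ReboundGameMode's game and round start/end and player death, throw, charge and pickup events.
; Each handler skips if Audio is playing, otherwise prints a random line, prefixed with the player's name for player events.
; Each printed line restarts a self-looping retriggerable delay, so interlude lines fill quiet spells.
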(event `self.ReceiveBeginPlay`
  (bind _asrebound_game_mode (cast `/Game/BluePrints/Gamemodes/ReboundGameMode` (`GameplayStatics.GetGameMode`)))
  (add `/Game/BluePrints/Gamemodes/ReboundGameMode.StartGame` _asrebound_game_mode (delegate `playStartGame`))
  (add `/Game/BluePrints/Gamemodes/ReboundGameMode.StartRound` _asrebound_game_mode (delegate `playStartRound`))
  (add `/Game/BluePrints/Gamemodes/ReboundGameMode.EndRound` _asrebound_game_mode (delegate `playEndRound`))
  (add `/Game/BluePrints/Gamemodes/ReboundGameMode.EndGame` _asrebound_game_mode (delegate `playEndGame`))
  (add `/Game/BluePrints/Gamemodes/ReboundGameMode.commDied` _asrebound_game_mode (delegate `playDied`))
  (add `/Game/BluePrints/Gamemodes/ReboundGameMode.commThrow` _asrebound_game_mode (delegate `playThrow`))
  (add `/Game/BluePrints/Gamemodes/ReboundGameMode.commCharge` _asrebound_game_mode (delegate `playCharge`))
  (add `/Game/BluePrints/Gamemodes/ReboundGameMode.commPickup` _asrebound_game_mode (delegate `playPickup`))
  (`self.PlayInterlude`))

(event `PlayInterlude`
  (bind _interlude (`self.Interlude`))
  ;[1 1 1] interlude
  (`KismetSystemLibrary.RetriggerableDelay` (`self.InterludeTime`))
  (`KismetSystemLibrary.PrintString` (`KismetArrayLibrary.Array_Get` _interlude (`KismetMathLibrary.RandomIntegerInRange` 0 (`KismetArrayLibrary.Array_Length` _interlude))) true true (struct :`G` 0.969 :`B` 0.733852 :`A` 1.0) 5.0)
  (`self.PlayInterlude`))

(event `playStartGame`
  (bind _gamestart (`self.GameStart`))
  ;[1 1 1] start game
  (if (not (`AudioComponent.IsPlaying` (`self.Audio`)))
    (`KismetSystemLibrary.PrintString` (`KismetArrayLibrary.Array_Get` _gamestart (`KismetMathLibrary.RandomIntegerInRange` 0 (`KismetArrayLibrary.Array_Length` _gamestart))) true true (struct :`G` 0.969 :`B` 0.733852 :`A` 1.0) 5.0)
    (`self.PlayInterlude`)))

(event `playEndRound`
  (bind _roundend (`self.RoundEnd`))
  ;[1 1 1] end round
  (if (not (`AudioComponent.IsPlaying` (`self.Audio`)))
    (`KismetSystemLibrary.PrintString` (`KismetArrayLibrary.Array_Get` _roundend (`KismetMathLibrary.RandomIntegerInRange` 0 (`KismetArrayLibrary.Array_Length` _roundend))) true true (struct :`G` 0.969 :`B` 0.733852 :`A` 1.0) 5.0)
    (`self.PlayInterlude`)))

(event `playDied`
  (params (ID :type Integer))
  (bind _playerdied (`self.PlayerDied`))
  ;[1 1 1] playerDied
  (if (not (`AudioComponent.IsPlaying` (`self.Audio`)))
    (`KismetSystemLibrary.PrintString` (`KismetStringLibrary.Concat_StrStr` (`KismetArrayLibrary.Array_Get` (`self.Players`) ID) (`KismetArrayLibrary.Array_Get` _playerdied (`KismetMathLibrary.RandomIntegerInRange` 0 (`KismetArrayLibrary.Array_Length` _playerdied)))))
    (`self.PlayInterlude`)))

(event `playCharge`
  (params (ID :type Integer))
  (bind _playercharge (`self.PlayerCharge`))
  ;[1 1 1] playerCharge
  (if (not (`AudioComponent.IsPlaying` (`self.Audio`)))
    (`KismetSystemLibrary.PrintString` (`KismetStringLibrary.Concat_StrStr` (`KismetArrayLibrary.Array_Get` (`self.Players`) ID) (`KismetArrayLibrary.Array_Get` _playercharge (`KismetMathLibrary.RandomIntegerInRange` 0 (`KismetArrayLibrary.Array_Length` _playercharge)))))
    (`self.PlayInterlude`)))

(event `playStartRound`
  (bind _roundstart (`self.RoundStart`))
  ;[1 1 1] start round
  (if (not (`AudioComponent.IsPlaying` (`self.Audio`)))
    (`KismetSystemLibrary.PrintString` (`KismetArrayLibrary.Array_Get` _roundstart (`KismetMathLibrary.RandomIntegerInRange` 0 (`KismetArrayLibrary.Array_Length` _roundstart))) true true (struct :`G` 0.969 :`B` 0.733852 :`A` 1.0) 5.0)
    (`self.PlayInterlude`)))

(event `playEndGame`
  (bind _gameend (`self.GameEnd`))
  ;[1 1 1] play end game
  (if (not (`AudioComponent.IsPlaying` (`self.Audio`)))
    (`KismetSystemLibrary.PrintString` (`KismetArrayLibrary.Array_Get` _gameend (`KismetMathLibrary.RandomIntegerInRange` 0 (`KismetArrayLibrary.Array_Length` _gameend))) true true (struct :`G` 0.969 :`B` 0.733852 :`A` 1.0) 5.0)
    (`self.PlayInterlude`)))

(event `playThrow`
  (params (ID :type Integer))
  (bind _playerthrow (`self.PlayerThrow`))
  ;[1 1 1] playerThrow
  (if (not (`AudioComponent.IsPlaying` (`self.Audio`)))
    (`KismetSystemLibrary.PrintString` (`KismetStringLibrary.Concat_StrStr` (`KismetArrayLibrary.Array_Get` (`self.Players`) ID) (`KismetArrayLibrary.Array_Get` _playerthrow (`KismetMathLibrary.RandomIntegerInRange` 0 (`KismetArrayLibrary.Array_Length` _playerthrow)))))
    (`self.PlayInterlude`)))

(event `playPickup`
  (params (ID :type Integer))
  (bind _playerpickup (`self.PlayerPickup`))
  ;[1 1 1] playerPickup
  (if (not (`AudioComponent.IsPlaying` (`self.Audio`)))
    (`KismetSystemLibrary.PrintString` (`KismetStringLibrary.Concat_StrStr` (`KismetArrayLibrary.Array_Get` (`self.Players`) ID) (`KismetArrayLibrary.Array_Get` _playerpickup (`KismetMathLibrary.RandomIntegerInRange` 0 (`KismetArrayLibrary.Array_Length` _playerpickup)))))
    (`self.PlayInterlude`)))

(fn `UserConstructionScript`)