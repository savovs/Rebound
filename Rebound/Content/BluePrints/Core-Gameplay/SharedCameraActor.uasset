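; Shared camera actor that becomes the view target for up to four players and follows every ReboundPlayerCharacter.
; Each tick it smoothly interpolates toward the characters' average XY position plus an offset.
; Its height lerps from a low offset up to its starting Z, using the largest horizontal gap between characters relative to the largest gap between PlayerStarts, recorded at BeginPlay.
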(event EventBeginPlay
  (for _index (range 0 3)
    (if (!= (Game|GetPlayerController _index) 0)
      (Game|Player|SetViewTargetwithBlend (Game|GetPlayerController _index) self 0.0 "VTBlend_Linear" 0.0 false)
      (bind _maxdistance (CallFunction|GetMaxDistance "/Script/Engine.PlayerStart"))
      (Variables|Default|SetMaxDistance _maxdistance)
      (Variables|Default|SetStartingPosition (Transformation|GetActorLocation)))))

(event EventTick
  (params (DeltaSeconds :type Float%20%28single-precision%29))
  (bind (_xpos _ypos) (CallFunction|AverageLocation))
  (bind _maxdistance (CallFunction|GetMaxDistance "/Game/BluePrints/Core-Gameplay/Characters/ReboundPlayerCharacter.ReboundPlayerCharacter_C"))
  (bind _zpos (CallFunction|DynamicZoom _maxdistance))
  (bind _output_get (Variables|Default|SetCurrentPos (Math|Vector|MakeVector _xpos _ypos _zpos)))
  (Transformation|SetActorLocation (Math|Interpolation|VInterpTo (Transformation|GetActorLocation) _output_get DeltaSeconds 3.0) false false))

(fn ConstructionScript)

(fn AverageLocation
  (bind _outactors (Actor|GetAllActorsOfClass "/Game/BluePrints/Core-Gameplay/Characters/ReboundPlayerCharacter.ReboundPlayerCharacter_C"))
  (for _array_element _outactors
    (LocalVariables|SetTotalLocTemp (+ (Transformation|GetActorLocation _array_element) (LocalVariables|GetTotalLocTemp))))
  (bind _output_get (LocalVariables|SetTotalLocTemp (Math|Vector|MakeVector (.x (/ (LocalVariables|GetTotalLocTemp) (Utilities|Array|Length _outactors))) (.y (/ (LocalVariables|GetTotalLocTemp) (Utilities|Array|Length _outactors))) (.z (Transformation|GetActorLocation)))))
  (return (.x (+ _output_get (Variables|Default|GetStandardOffset))) (.y (+ _output_get (Variables|Default|GetStandardOffset)))))

(fn DynamicZoom
  (params (CurMaxDistance :type Float%20%28single-precision%29))
  (return (Math|Float|Lerp (+ (.z (Variables|Default|GetStartingPosition)) (Variables|Default|GetLowestPositionOffset)) (.z (Variables|Default|GetStartingPosition)) (/ CurMaxDistance (Variables|Default|GetMaxDistance)))))

(fn GetMaxDistance
  (params (Class :type Actor%20Class%20Reference))
  (bind _distances (LocalVariables|GetDistances))
  (bind _outactors (Actor|GetAllActorsOfClass Class))
  (for _array_element _outactors
    (for _array_element_2 _outactors
      (Utilities|Array|Add _distances (Transformation|GetHorizontalDistanceTo _array_element _array_element_2))))
  (return (.MaxValue (Math|Float|MaxOfFloatArray _distances))))