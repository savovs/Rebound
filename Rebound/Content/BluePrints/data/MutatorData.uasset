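; MutatorData spawns the active gameplay mutator for the session when play begins.
; It reads the PersistentData game instance and, if LoadData is set, spawns the MutatorsList class indexed by PlaylistID.
; Otherwise it spawns the TestMutators class as a fallback.
; The spawned actor is placed at the world origin and stored in ActiveMutators; nothing spawns if the game instance cast fails.
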(event `self.ReceiveBeginPlay`
  ;[1 1 1] bind events
  (`self.SpawnMutators`))

(fn `SpawnMutators`
  (bind _returnvalue (`KismetMathLibrary.MakeTransform` (0.0 0.0 0.0)))
  (bind _activemutators (`self.activeMutators`))
  (bind _aspersistent_data (cast `/Game/BluePrints/data/PersistentData` (`GameplayStatics.GetGameInstance`)))
  (if (`/Game/BluePrints/data/PersistentData.loadData` _aspersistent_data)
    (bind _returnvalue_2 (`|SpawnActorFromClass` (`KismetArrayLibrary.Array_Get` (`/Game/BluePrints/data/PersistentData.MutatorsList` _aspersistent_data) (`/Game/BluePrints/data/PersistentData.playlistID` _aspersistent_data)) _returnvalue "Undefined" "OverrideRootScale"))
    (`KismetArrayLibrary.Array_Add` _activemutators _returnvalue_2)
    (else
      (bind _returnvalue_3 (`|SpawnActorFromClass` (`self.testMutators`) _returnvalue "Undefined" "OverrideRootScale"))
      (`KismetArrayLibrary.Array_Add` _activemutators _returnvalue_3))))

(fn `UserConstructionScript`)