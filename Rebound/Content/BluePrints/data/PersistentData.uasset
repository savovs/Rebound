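; PersistentData holds and applies the game's video settings, forcing Medium graphics quality on Init.
; OverallGraphicsChange stores the chosen preset and runs console commands for post-processing, shadows, textures and effects, built by appending a level to stored command strings.
; Low keeps shadows at the same level as Medium.
; FullscreenToggle switches screen mode by console command and tracks it in a boolean.
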(event `self.ReceiveInit`
  (`self.OverallGraphicsChange` "NewEnumerator1"))

(fn `FullscreenToggle`
  (if (`self.isFullscreen`)
    (`KismetSystemLibrary.ExecuteConsoleCommand` "fullscreen 0")
    (set `self.isFullscreen` false)
    (else
      (`KismetSystemLibrary.ExecuteConsoleCommand` "fullscreen 2")
      (set `self.isFullscreen` true))))

(fn `OverallGraphicsChange`
  (params (Graphics :type "/Game/BluePrints/data/GraphicsQuality Enum"))
  (bind _output_get (set `self.OverallGraphicsQuality` Graphics))
  (switch `/Game/BluePrints/data/GraphicsQuality` _output_get
    (:`NewEnumerator0`
      (`KismetSystemLibrary.ExecuteConsoleCommand` (`KismetStringLibrary.Concat_StrStr` (`self.PostProcessing`) "0"))
      (`KismetSystemLibrary.ExecuteConsoleCommand` (`KismetStringLibrary.Concat_StrStr` (`self.ShadowQuality`) "1"))
      (`KismetSystemLibrary.ExecuteConsoleCommand` (`KismetStringLibrary.Concat_StrStr` (`self.TextureQuality`) "0"))
      (`KismetSystemLibrary.ExecuteConsoleCommand` (`KismetStringLibrary.Concat_StrStr` (`self.EffectsQuality`) "0"))
      (`KismetSystemLibrary.PrintString` "Graphics Set To Low" false))
    (:`NewEnumerator1`
      (`KismetSystemLibrary.ExecuteConsoleCommand` (`KismetStringLibrary.Concat_StrStr` (`self.PostProcessing`) "1"))
      (`KismetSystemLibrary.ExecuteConsoleCommand` (`KismetStringLibrary.Concat_StrStr` (`self.ShadowQuality`) "1"))
      (`KismetSystemLibrary.ExecuteConsoleCommand` (`KismetStringLibrary.Concat_StrStr` (`self.TextureQuality`) "1"))
      (`KismetSystemLibrary.ExecuteConsoleCommand` (`KismetStringLibrary.Concat_StrStr` (`self.EffectsQuality`) "1"))
      (`KismetSystemLibrary.PrintString` "Graphics Set To Medium" false))
    (:`NewEnumerator2`
      (`KismetSystemLibrary.ExecuteConsoleCommand` (`KismetStringLibrary.Concat_StrStr` (`self.PostProcessing`) "2"))
      (`KismetSystemLibrary.ExecuteConsoleCommand` (`KismetStringLibrary.Concat_StrStr` (`self.ShadowQuality`) "2"))
      (`KismetSystemLibrary.ExecuteConsoleCommand` (`KismetStringLibrary.Concat_StrStr` (`self.TextureQuality`) "2"))
      (`KismetSystemLibrary.ExecuteConsoleCommand` (`KismetStringLibrary.Concat_StrStr` (`self.EffectsQuality`) "2"))
      (`KismetSystemLibrary.PrintString` "Graphics Set To High" false))
    (:`NewEnumerator3`
      (`KismetSystemLibrary.ExecuteConsoleCommand` (`KismetStringLibrary.Concat_StrStr` (`self.PostProcessing`) "3"))
      (`KismetSystemLibrary.ExecuteConsoleCommand` (`KismetStringLibrary.Concat_StrStr` (`self.ShadowQuality`) "3"))
      (`KismetSystemLibrary.ExecuteConsoleCommand` (`KismetStringLibrary.Concat_StrStr` (`self.TextureQuality`) "3"))
      (`KismetSystemLibrary.ExecuteConsoleCommand` (`KismetStringLibrary.Concat_StrStr` (`self.EffectsQuality`) "3"))
      (`KismetSystemLibrary.PrintString` "Graphics Set To Epic" false))))