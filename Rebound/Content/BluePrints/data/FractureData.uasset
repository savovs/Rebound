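; FractureData snapshots the level's fracturable walls and restores them each time a round starts.
; On BeginPlay it binds to the ReboundGameMode round-start event and records every WallBP's class, transform and fracture stats, plus wall stats for MovingWallBP instances, in index-matched arrays.
; On round start it destroys all walls, respawns them from those arrays, reapplies their stats and calls StatsAssigned on each.
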(event `self.ReceiveBeginPlay`
  (bind _asrebound_game_mode (cast `/Game/BluePrints/Gamemodes/ReboundGameMode` (`GameplayStatics.GetGameMode`)))
  (add `/Game/BluePrints/Gamemodes/ReboundGameMode.startRound` _asrebound_game_mode (delegate `start Round`))
  (`self.getFractureTransforms`)
  (`KismetSystemLibrary.PrintString` (`KismetStringLibrary.TimeSecondsToString` (`KismetSystemLibrary.GetGameTimeInSeconds`))))

(event `start Round`
  (`KismetSystemLibrary.PrintString` "bind working" true true (struct :`R` 1.0 :`G` 0.296274 :`A` 1.0))
  (`self.resetFractures`))

(fn `getFractureTransforms`
  (bind _walltrans (`self.WallTrans`))
  (bind _outactors (`GameplayStatics.GetAllActorsOfClass` "/Game/BluePrints/enviroment/Walls/WallBP.WallBP_C"))
  (for _array_element _outactors
    (`KismetArrayLibrary.Array_Add` (`self.WallClass`) (`GameplayStatics.GetObjectClass` _array_element))
    (bind _returnvalue (`KismetArrayLibrary.Array_Add` _walltrans (`self.GetTransform` _array_element)))
    (`KismetArrayLibrary.Array_Add` (`self.FractureStats`) (`/Game/BluePrints/enviroment/Walls/WallBP.FractureStats` _array_element))
    (bind _asmoving_wall_bp (cast `/Game/BluePrints/enviroment/Walls/MovingWallBP` _array_element))
    (`KismetSystemLibrary.PrintString` "moving wall" true true (struct :`R` 0.10593 :`G` 1.0 :`B` 0.065227 :`A` 1.0))
    (`KismetArrayLibrary.Array_Set` (`self.WallStats`) _returnvalue (`/Game/BluePrints/enviroment/Walls/MovingWallBP.WallStats` _asmoving_wall_bp) true))
  (`KismetSystemLibrary.PrintString` (`KismetStringLibrary.BuildString_Int` "" "total fractures " (`KismetArrayLibrary.Array_Length` _walltrans) "  ") true true (struct :`R` 0.166948 :`G` 1.0 :`A` 1.0)))

(fn `resetFractures`
  (bind _outactors (`GameplayStatics.GetAllActorsOfClass` "/Game/BluePrints/enviroment/Walls/WallBP.WallBP_C"))
  (for _array_element _outactors
    (`self.K2_DestroyActor` _array_element))
  (for (_array_element_2 _array_index) (`self.WallClass`)
    (bind _returnvalue (`|SpawnActorFromClass` _array_element_2 (`KismetArrayLibrary.Array_Get` (`self.WallTrans`) _array_index) "Undefined" "OverrideRootScale"))
    (`|ExecutionSequence`
      (:`then_0`
        (set `/Game/BluePrints/enviroment/Walls/WallBP.FractureStats` (`KismetArrayLibrary.Array_Get` (`self.FractureStats`) _array_index) _returnvalue))
      (:`then_1`
        (bind _asmoving_wall_bp (cast `/Game/BluePrints/enviroment/Walls/MovingWallBP` _returnvalue))
        (set `/Game/BluePrints/enviroment/Walls/MovingWallBP.WallStats` (`KismetArrayLibrary.Array_Get` (`self.WallStats`) _array_index) _asmoving_wall_bp))
      (:`then_2`
        (`/Game/BluePrints/enviroment/Walls/WallBP.StatsAssigned` _returnvalue))))
  (`KismetSystemLibrary.PrintString` (`KismetStringLibrary.BuildString_Int` "" "spawned " _array_index "actors")))

(fn `UserConstructionScript`)