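; End-of-game mode that shows the EndGameUI widget and arranges the podiums by each player's win count.
; On BeginPlay it ranks four player slots from PersistentData's Wins by repeated max extraction, overwriting matched scores with a sentinel so tied players resolve separately.
; It then sets up the level's PodiumSetUp podiums in rank order, giving tied scores a shared position and hiding podiums for absent players.
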(event EventBeginPlay
  (bind _scoressorted (Variables|Default|GetScoresSorted))
  (bind _returnvalue (UserInterface|CreateWidget "/Game/UI/InGame/EndGameUI.EndGameUI_C"))
  (UserInterface|Viewport|AddtoViewport _returnvalue 0)
  (bind _aspersistent_data (Utilities|Casting|CastToPersistentData (Game|GetGameInstance)))
  (bind _output_get (Variables|Default|SetPersisData _aspersistent_data))
  (Variables|Default|SetGlobalTempScor (Variables|/Game/BluePrints/data/PersistentData.PersistentData_C|GetWins _output_get))
  (for _index (range 0 3)
    ;[1 1 1] set the players in ofder
    (bind _score (CallFunction|GetScoreatRank _index))
    (bind _playernum (CallFunction|GetPlayeratScore _score))
    (Utilities|Array|Insert (Variables|Default|GetPlayerRanking) _playernum _index))
  (bind _outactors (Actor|GetAllActorsOfClass "/Game/BluePrints/enviroment/PodiumSetUp.PodiumSetUp_C"))
  (for (_array_element _array_index) (Variables|/Game/BluePrints/enviroment/PodiumSetUp.PodiumSetUp_C|GetPodiums (Utilities|Array|Get(acopy) _outactors))
    (if (== (Utilities|Array|Get(acopy) (Variables|/Game/BluePrints/data/PersistentData.PersistentData_C|GetPlayers _aspersistent_data) (Utilities|Array|Get(acopy) (Variables|Default|GetPlayerRanking) _array_index)) -1)
      ;[1 1 1] no player
      (Rendering|SetActorHiddenInGame _array_element true)
      (Development|PrintString "hide pod" (Variables|/Game/BluePrints/data/PersistentData.PersistentData_C|GetisDevMode (Variables|Default|GetpersisData)))
      (elif (== _array_index 0)
        ;[1 1 1] set first player as 1
        (Default|SetUpPodium _array_element 0 (Utilities|Array|Get(acopy) (Variables|Default|GetPlayerRanking) _array_index))
        (Variables|Default|SetlastPos 0)
        (Development|PrintString "first player" (Variables|/Game/BluePrints/data/PersistentData.PersistentData_C|GetisDevMode (Variables|Default|GetpersisData)))
        (elif (== (Utilities|Array|Get(acopy) _scoressorted _array_index) (Utilities|Array|Get(acopy) _scoressorted (- _array_index 1)))
          ;[1 1 1] set draw
          (Default|SetUpPodium _array_element (Variables|Default|GetlastPos) (Utilities|Array|Get(acopy) (Variables|Default|GetPlayerRanking) _array_index))
          (Development|PrintString "draw index" (Variables|/Game/BluePrints/data/PersistentData.PersistentData_C|GetisDevMode (Variables|Default|GetpersisData)))
          (else
            (bind _result (Math|Integer|IncrementInt (Variables|Default|GetlastPos))
              (:%20%20
                ;[1 1 1] set next
                (Default|SetUpPodium _array_element _result (Utilities|Array|Get(acopy) (Variables|Default|GetPlayerRanking) _array_index))
                (Development|PrintString "next player" (Variables|/Game/BluePrints/data/PersistentData.PersistentData_C|GetisDevMode (Variables|Default|GetpersisData)))))))))))

(event EventTick
  (params (DeltaSeconds :type Float%20%28single-precision%29)))

(fn ConstructionScript)

(fn GetScoreatRank
  (params (Rank :type Integer))
  (bind _output_get (LocalVariables|SetTempoaryScores (Variables|/Game/BluePrints/data/PersistentData.PersistentData_C|GetWins (Variables|Default|GetPersisData))))
  (for _index (range 0 Rank)
    (LocalVariables|SetTempScore (.MaxValue (Math|Integer|MaxOfIntArray _output_get)))
    (Utilities|Array|RemoveIndex (LocalVariables|GetTempoaryScores) (.IndexOfMaxValue (Math|Integer|MaxOfIntArray _output_get))))
  (Utilities|Array|SetArrayElem (Variables|Default|GetScoresSorted) Rank (LocalVariables|GetTempScore) true)
  (return (LocalVariables|GetTempScore)))

(fn GetPlayeratScore
  (params (Score :type Integer))
  (bind _globaltempscor (Variables|Default|GetGlobalTempScor))
  (bind _returnvalue (Utilities|Array|FindItem _globaltempscor Score))
  (bind _output_get (LocalVariables|SetTempValue _returnvalue))
  (Utilities|Array|SetArrayElem _globaltempscor _returnvalue -100)
  (return _output_get))