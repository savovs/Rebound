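; Moving wall that toggles between up and down heights from its WallStats, unless fractured.
; Toggles come from the first FractureData actor, plus either a DodgeBall leaving its sphere trigger or bound pressure plates, depending on UseTrigger.
; Tick lerps height at constant speed with actor collision off until arrival, holding the trigger sphere at the up height.
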(event `self.StatsAssigned`
  (bind _returnvalue_location (`KismetMathLibrary.BreakTransform` (`self.GetTransform`)))
  (bind _wallstats_startingposup (break `/Game/BluePrints/enviroment/WallStats` (`self.WallStats`)))
  (bind (_wallstats_startingposup_2 _wallstats_uppoint _wallstats_downpoint _wallstats_speed _wallstats_pressureplates _wallstats_triggersize) (break `/Game/BluePrints/enviroment/WallStats` (`self.WallStats`)))
  (bind (_wallstats_startingposup_3 _wallstats_uppoint_2 _wallstats_downpoint_2) (break `/Game/BluePrints/enviroment/WallStats` (`self.WallStats`)))
  (bind (_wallstats_startingposup_4 _wallstats_uppoint_3 _wallstats_downpoint_3 _wallstats_speed_2 _wallstats_pressureplates_2 _wallstats_triggersize_2 _wallstats_usetrigger) (break `/Game/BluePrints/enviroment/WallStats` (`self.WallStats`)))
  (bind (_returnvalue_x _returnvalue_y) (`KismetMathLibrary.BreakVector` (`SceneComponent.K2_GetComponentScale` (`self.DefaultSceneRoot`))))
  (`parent.StatsAssigned`)
  (set `self.distance` (`KismetMathLibrary.VSize` (- _wallstats_uppoint_2 _wallstats_downpoint_2)))
  (bind _outactors (`GameplayStatics.GetAllActorsOfClass` "/Game/BluePrints/data/FractureData.FractureData_C"))
  (add `/Game/BluePrints/data/FractureData.ToggleWall` (`KismetArrayLibrary.Array_Get` _outactors) (delegate `Toggle wall`))
  (if (not _wallstats_startingposup)
    (`self.toggleWall`))
  (if _wallstats_usetrigger
    (`SphereComponent.SetSphereRadius` (`self.SphereCollider`) _wallstats_triggersize true)
    (`KismetSystemLibrary.DrawDebugSphere` _returnvalue_location (* _returnvalue_y _wallstats_triggersize) 12 (struct :`R` 1.0 :`G` 1.0 :`B` 1.0 :`A` 1.0) 5.0)
    (else
      (for _array_element _wallstats_pressureplates_2
        (add `/Game/BluePrints/enviroment/wallPressurePlate.ToggleWall` _array_element (delegate `Toggle wall`)))
      (`SphereComponent.SetSphereRadius` (`self.SphereCollider`) 0.0 true))))

(event `self.ReceiveTick`
  (params (DeltaSeconds :type "Float (single-precision)"))
  (`parent.ReceiveTick` DeltaSeconds)
  (if (`self.moveWall`)
    (`self.moveWallUp`)))

(event `self.SphereCollider.OnComponentEndOverlap`
  (params (OtherActor :type "Actor Object Reference") (OtherComp :type "PrimitiveComponent Object Reference") (OtherBodyIndex :type Integer))
  (cast `/Game/BluePrints/Core-Gameplay/Dodgeballs/DodgeBall` OtherActor)
  (`self.toggleWall`))

(event `Toggle wall`
  (`self.toggleWall`))

(fn `moveWallUp`
  (bind (_wallstats_startingposup _wallstats_uppoint) (break `/Game/BluePrints/enviroment/WallStats` (`self.WallStats`)))
  (bind (_wallstats_startingposup_2 _wallstats_uppoint_2 _wallstats_downpoint) (break `/Game/BluePrints/enviroment/WallStats` (`self.WallStats`)))
  (bind (_wallstats_startingposup_3 _wallstats_uppoint_3 _wallstats_downpoint_2 _wallstats_speed) (break `/Game/BluePrints/enviroment/WallStats` (`self.WallStats`)))
  (bind _returnvalue (/ (* (- (`KismetSystemLibrary.GetGameTimeInSeconds`) (`self.startTime`)) _wallstats_speed) (`self.distance`)))
  (`self.K2_SetActorTransform` (`KismetMathLibrary.TLerp` (`self.starting point`) (`KismetMathLibrary.MakeTransform` (`KismetMathLibrary.MakeVector` (.x (.location (`self.GetTransform`))) (.y (.location (`self.GetTransform`))) (.z (`KismetMathLibrary.SelectVector` _wallstats_uppoint_2 _wallstats_downpoint (`self.CurPosUp`)))) (.rotation (`self.GetTransform`)) (.scale (`self.GetTransform`))) _returnvalue))
  (`SceneComponent.K2_SetWorldLocation` (`self.SphereCollider`) (`KismetMathLibrary.MakeVector` (.x (`self.K2_GetActorLocation`)) (.y (`self.K2_GetActorLocation`)) (.z _wallstats_uppoint)) false false)
  (if (>= _returnvalue 1.0)
    (set `self.moveWall` false)
    (`self.SetActorEnableCollision` true)))

(fn `toggleWall`
  (if (not (`self.isFractured`))
    (set `self.CurPosUp` (not (`self.CurPosUp`)))
    (set `self.moveWall` true)
    (set `self.starting point` (`self.GetTransform`))
    (set `self.startTime` (`KismetSystemLibrary.GetGameTimeInSeconds`))
    (`self.SetActorEnableCollision` false)))

(fn `UserConstructionScript`
  (`parent.UserConstructionScript`))