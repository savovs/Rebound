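; PodiumSetUp is an environment actor that stages the end-of-level podium showing players in ranked order.
; On BeginPlay it blends the first player controller's view to its Camera, if valid.
; SetPodiums, not called within this Blueprint, reads PlayerRanking from EndLevelMode and spawns an idle-animated character mesh at each matching podium position.
; Each mesh gets a dynamic material instance tinted with that player's colour from persistent data.
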(event `self.ReceiveBeginPlay`
  (bind _camera (`self.Camera`))
  (`/Engine/EditorBlueprintResources/StandardMacros.IsValid` _camera
    (:`Is Valid`
      (`PlayerController.SetViewTargetWithBlend` (`GameplayStatics.GetPlayerController` 0) _camera 0.0 "VTBlend_Linear" 0.0 false))))

(fn `SetPodiums`
  (bind _asend_level_mode (cast `/Game/BluePrints/Gamemodes/EndLevelMode` (`GameplayStatics.GetGameMode`)))
  (for (_array_element _array_index) (`/Game/BluePrints/Gamemodes/EndLevelMode.PlayerRanking` _asend_level_mode)
    (bind _returnvalue (`|SpawnActorFromClass` "/Script/Engine.SkeletalMeshActor" (`self.GetTransform` (`KismetArrayLibrary.Array_Get` (`self.PodiumPositions`) _array_index)) "Undefined" "OverrideRootScale"))
    (bind _skeletalmeshcomponent (`SkeletalMeshActor.SkeletalMeshComponent` _returnvalue))
    (`SkinnedMeshComponent.SetSkinnedAssetAndUpdate` _skeletalmeshcomponent "/Game/Art/Character/Character_new/Character_rigged.Character_rigged")
    (`SkeletalMeshComponent.PlayAnimation` _skeletalmeshcomponent "/Game/Art/Character/Animations/Idle_001.Idle_001" true)
    (bind _returnvalue_2 (`PrimitiveComponent.CreateDynamicMaterialInstance` _skeletalmeshcomponent 0 "/Game/Art/Character/Character_new/playerColourInstance.playerColourInstance"))
    (bind _item_charcolour (break `/Game/BluePrints/Core-Gameplay/Characters/CustomCharacterStats` (`KismetArrayLibrary.Array_Get` (`/Game/BluePrints/data/PersistentData.PlayerCharacters` (`/Game/BluePrints/Gamemodes/EndLevelMode.PersistentData` _asend_level_mode)) _array_element)))
    (`MaterialInstanceDynamic.SetVectorParameterValue` _returnvalue_2 "playerColour" _item_charcolour))
  (`KismetSystemLibrary.PrintString` "Complete"))

(fn `UserConstructionScript`)