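; Pressure plate Blueprint that signals a wall toggle when players step on or off it.
; Begin and end overlaps on its Box respond only to ReboundPlayerCharacter actors.
; Counting overlapping players makes ToggleWall fire only when the first arrives or the last leaves, so additional players on the plate do not re-toggle it.
; Both transitions share the same ToggleWall call, with no on/off state passed; the wall's response is defined outside this graph.
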(event `self.Box.OnComponentEndOverlap`
  (params (OtherActor :type "Actor Object Reference") (OtherComp :type "PrimitiveComponent Object Reference") (OtherBodyIndex :type Integer))
  (cast `/Game/BluePrints/Core-Gameplay/Characters/ReboundPlayerCharacter` OtherActor)
  (if (== (`KismetArrayLibrary.Array_Length` (`PrimitiveComponent.GetOverlappingActors` (`self.Box`) "/Game/BluePrints/Core-Gameplay/Characters/ReboundPlayerCharacter.ReboundPlayerCharacter_C")) 0)
    (`self.ToggleWall` :!label _label)))

(event `self.Box.OnComponentBeginOverlap`
  (params (OtherActor :type "Actor Object Reference") (OtherComp :type "PrimitiveComponent Object Reference") (OtherBodyIndex :type Integer) (bFromSweep :type Boolean) (SweepResult :type "HitResult Structure (by ref)"))
  (cast `/Game/BluePrints/Core-Gameplay/Characters/ReboundPlayerCharacter` OtherActor)
  (if (== (`KismetArrayLibrary.Array_Length` (`PrimitiveComponent.GetOverlappingActors` (`self.Box`) "/Game/BluePrints/Core-Gameplay/Characters/ReboundPlayerCharacter.ReboundPlayerCharacter_C")) 1)
    (goto _label)))

(fn `UserConstructionScript`)