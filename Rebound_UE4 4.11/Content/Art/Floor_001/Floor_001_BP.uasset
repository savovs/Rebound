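; Floor actor Blueprint that changes its emissive light to a random bright colour every second.
; BeginPlay starts a looping timer that calls SetLightColour.
; Each call creates a fresh dynamic material instance on the Floor, sets a fixed Brightness and feeds randomised, overbright RGB into LightColour.
; Debug strings print on each change, one in a re-randomised colour that need not match the floor.
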(event `self.ReceiveBeginPlay`
  (`KismetSystemLibrary.K2_SetTimer` self "SetLightColour" 1.0 true))

(event `self.ReceiveTick`
  (params (DeltaSeconds :type "Float (single-precision)")))

(fn `setLightColour`
  (bind _linearcolor (make `LinearColor` (`KismetMathLibrary.Lerp` 0.0 100.0 (+ 0.0 (`KismetMathLibrary.RandomFloatInRange` 0.0 1.0))) (`KismetMathLibrary.Lerp` 0.0 100.0 (+ 0.0 (`KismetMathLibrary.RandomFloatInRange` 0.0 1.0))) (`KismetMathLibrary.Lerp` 0.0 100.0 (+ 0.0 (`KismetMathLibrary.RandomFloatInRange` 0.0 1.0))) 1.0))
  (`KismetSystemLibrary.PrintString` "Hello")
  (bind _returnvalue (`PrimitiveComponent.CreateDynamicMaterialInstance` (`self.floor`) 0 "/Game/Art/Floor_001/Floor_001_emissive_mat2_Inst.Floor_001_emissive_mat2_Inst"))
  (`MaterialInstanceDynamic.SetScalarParameterValue` _returnvalue "Brightness" 10.0)
  (`MaterialInstanceDynamic.SetVectorParameterValue` _returnvalue "LightColour" _linearcolor)
  (`KismetSystemLibrary.PrintString` "Hello" true true _linearcolor))

(fn `UserConstructionScript`)