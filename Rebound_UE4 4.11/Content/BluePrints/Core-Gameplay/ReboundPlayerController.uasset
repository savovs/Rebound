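; Player controller for Rebound that handles spawning and possessing the player character, with game-and-UI input set on BeginPlay.
; Tick runs RespawnCheck, which advances and clamps a respawn timer while respawning is allowed and no pawn is controlled, then only casts the game mode without requesting a spawn.
; SpawnPawn, not called within this file, spawns a ReboundPlayerCharacter at a given transform if pawnless, possesses it and sets its token colour.
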(event `self.ReceiveBeginPlay`
  (`WidgetBlueprintLibrary.SetInputMode_GameAndUIEx` null))

(event `self.ReceiveTick`
  (params (DeltaSeconds :type "Float (single-precision)"))
  (`self.RespawnCheck`))

(fn `RespawnCheck`
  (if (`self.CanRespawn`)
    (if (== (`self.K2_GetPawn`) null)
      (bind _output_get (set `self.RespawnTimerCur` (+ (`self.RespawnTimerCur`) (`GameplayStatics.GetWorldDeltaSeconds`))))
      (if (>= _output_get (`self.RespawnTimerMax`))
        (set `self.RespawnTimerCur` (`self.RespawnTimerMax`))
        (cast `/Game/BluePrints/Gamemodes/ReboundGameMode` (`GameplayStatics.GetGameMode`))))))

(fn `SpawnPawn`
  (params (SpawnPoint :type "Transform Structure"))
  (if (== (`self.K2_GetPawn`) null)
    (bind _returnvalue (`|SpawnActorFromClass` "/Game/BluePrints/Core-Gameplay/ReboundPlayerCharacter.ReboundPlayerCharacter_C" SpawnPoint "Undefined" "OverrideRootScale"))
    (`self.Possess` _returnvalue)
    (`/Game/BluePrints/Core-Gameplay/ReboundPlayerCharacter.SetTokenColour` _returnvalue)))

(fn `UserConstructionScript`)