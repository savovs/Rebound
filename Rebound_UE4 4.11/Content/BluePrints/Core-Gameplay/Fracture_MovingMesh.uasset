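; A movable wall actor that shifts vertically between the heights of UpPoint and DownPoint.
; ToggleWall flips the target, records start transform and time, and disables collision; BeginPlay calls it once with a debug print.
; Tick runs MoveWallUp, lerping toward the target Z by elapsed time, Speed and the construction-time Distance.
; Movement stops and collision returns only when that lerp alpha reaches 100, not 1.
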(event `self.ReceiveBeginPlay`
  (`self.toggleWall`)
  (`KismetSystemLibrary.PrintString` "TEST"))

(event `self.ReceiveTick`
  (params (DeltaSeconds :type "Float (single-precision)"))
  (`parent.ReceiveTick` 0.0)
  (if (`self.moveWall`)
    (`self.moveWallUp`)))

(fn `moveWallUp`
  (bind _returnvalue (/ (* (- (`KismetSystemLibrary.GetGameTimeInSeconds`) (`self.startTime`)) (`self.speed`)) (`self.distance`)))
  (`self.K2_SetActorTransform` (`KismetMathLibrary.TLerp` (`self.starting point`) (`KismetMathLibrary.MakeTransform` (`KismetMathLibrary.MakeVector` (.x (.location (`self.GetTransform`))) (.y (.location (`self.GetTransform`))) (.z (`KismetMathLibrary.SelectVector` (`self.upPoint`) (`self.downPoint`) (`self.wallUp`)))) (.rotation (`self.GetTransform`)) (.scale (`self.GetTransform`))) _returnvalue))
  (if (>= _returnvalue 100.0)
    (set `self.moveWall` false)
    (`self.SetActorEnableCollision` true)))

(fn `toggleWall`
  (set `self.wallUp` (select `bool` (`self.wallUp`) :`false` true))
  (set `self.moveWall` true)
  (set `self.starting point` (`self.GetTransform`))
  (set `self.startTime` (`KismetSystemLibrary.GetGameTimeInSeconds`))
  (`self.SetActorEnableCollision` false))

(fn `UserConstructionScript`
  (`parent.UserConstructionScript`)
  (set `self.distance` (`KismetMathLibrary.VSize` (- (`self.upPoint`) (`self.downPoint`)))))