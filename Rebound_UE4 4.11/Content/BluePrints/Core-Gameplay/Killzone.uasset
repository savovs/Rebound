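; Killzone actor that acts as an arena boundary, killing players and removing dodgeballs that leave its box.
; On BeginPlay it binds to the box's end-overlap event, so the trigger fires on exit rather than entry.
; Exiting players are reported to ReboundGameMode as died, while exiting dodgeballs are destroyed through the game mode unless they are being carried.
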(event `self.ReceiveBeginPlay`
  (add `PrimitiveComponent.OnComponentEndOverlap` (`self.Box`) (delegate `OnComponentEndOverlap_Event_0`)))

(event `OnComponentEndOverlap_Event_0`
  (params (OtherActor :type "Actor Object Reference") (OtherComp :type "PrimitiveComponent Object Reference") (OtherBodyIndex :type Integer))
  (bind _asrebound_game_mode (cast `/Game/BluePrints/Gamemodes/ReboundGameMode` (`GameplayStatics.GetGameMode`)))
  (bind _asrebound_player_character (cast `/Game/BluePrints/Core-Gameplay/ReboundPlayerCharacter` OtherActor)
    (:`then`
      (`/Game/BluePrints/Gamemodes/ReboundGameMode.playerDied` _asrebound_game_mode 0 0 false _asrebound_player_character))
    (:`CastFailed`
      (bind _asdodge_ball (cast `/Game/BluePrints/Core-Gameplay/Dodgeballs/DodgeBall` OtherActor))
      (if (not (`/Game/BluePrints/Core-Gameplay/Dodgeballs/DodgeBall.IsCarried` _asdodge_ball))
        (`/Game/BluePrints/Gamemodes/ReboundGameMode.DestroyBall` _asrebound_game_mode _asdodge_ball)))))

(fn `UserConstructionScript`)