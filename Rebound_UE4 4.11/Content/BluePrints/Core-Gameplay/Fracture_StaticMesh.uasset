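; Destructible prop that fades out and removes itself after it fractures.
; The fracture event sets a flag and activates a particle system.
; While flagged, Tick lowers a Brightness value over time and pushes it to two material slots through dynamic instances of a wireframe material, created anew each frame.
; The actor destroys itself once brightness drops to a negative threshold.
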(event `self.ReceiveTick`
  (params (DeltaSeconds :type "Float (single-precision)"))
  (if (`self.isFractured`)
    (`self.ChangeBrightness` DeltaSeconds)))

(event `self.DestructibleComponent.OnComponentFracture`
  (params (HitPoint :type "Vector Structure (by ref)") (HitDirection :type "Vector Structure (by ref)"))
  (set `self.isFractured` true)
  (`ActorComponent.SetActive` (`self.ParticleSystem`) true false))

(fn `ChangeBrightness`
  (params (DeltaTime :type "Float (double-precision)"))
  (bind _destructiblecomponent (`self.DestructibleComponent`))
  (bind _output_get (set `self.Brightness` (- (`self.Brightness`) DeltaTime)))
  (bind _returnvalue (`PrimitiveComponent.CreateDynamicMaterialInstance` _destructiblecomponent 0 "/Game/Art/Wireframe_Inst.Wireframe_Inst"))
  (`MaterialInstanceDynamic.SetScalarParameterValue` _returnvalue "Brightness" _output_get)
  (bind _returnvalue_2 (`PrimitiveComponent.CreateDynamicMaterialInstance` _destructiblecomponent 1 "/Game/Art/Wireframe_Inst.Wireframe_Inst"))
  (`MaterialInstanceDynamic.SetScalarParameterValue` _returnvalue_2 "Brightness" _output_get)
  (if (<= _output_get -2.0)
    (`self.K2_DestroyActor`)))

(fn `UserConstructionScript`)