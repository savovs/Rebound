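; BallData manages dodgeball spawning and removal across Rebound rounds, following the game mode's start and end round events.
; Round start spawns the game mode's main ball at every active Ballspawn gathered on BeginPlay; round end destroys all DodgeBalls without resetting BallCount.
; During play, Tick tops up the count at random spawn points.
; DestroyABall decrements the count only for starter balls, so only their loss triggers replacements.
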(event `self.ReceiveBeginPlay`
  (`self.GetBallSpawns`)
  (bind _asrebound_game_mode (cast `/Game/BluePrints/Gamemodes/ReboundGameMode` (`GameplayStatics.GetGameMode`)))
  (add `/Game/BluePrints/Gamemodes/ReboundGameMode.StartRound` _asrebound_game_mode (delegate `StartRoundCall`))
  (add `/Game/BluePrints/Gamemodes/ReboundGameMode.EndRound` _asrebound_game_mode (delegate `EndRoundCall`)))

(event `StartRoundCall`
  (`self.SpawnBalls`)
  (set `self.Inplay` true))

(event `EndRoundCall`
  (`self.DespawnBalls`)
  (set `self.Inplay` false))

(event `self.ReceiveTick`
  (params (DeltaSeconds :type "Float (single-precision)"))
  (if (`self.Inplay`)
    (if (< (`self.BallCount`) (`KismetArrayLibrary.Array_Length` (`self.BallSpawns`)))
      (bind _asrebound_game_mode (cast `/Game/BluePrints/Gamemodes/ReboundGameMode` (`GameplayStatics.GetGameMode`)))
      (`self.SpawnABall` (`/Game/BluePrints/Gamemodes/ReboundGameMode.MainDodgeBall` _asrebound_game_mode))
      (`KismetSystemLibrary.PrintString` "respawn ball"))))

(fn `DespawnBalls`
  (bind _outactors (`GameplayStatics.GetAllActorsOfClass` "/Game/BluePrints/Core-Gameplay/Dodgeballs/DodgeBall.DodgeBall_C"))
  (for _array_element _outactors
    (`self.K2_DestroyActor` _array_element)))

(fn `DestroyABall`
  (params (BallDestroy :type "/Game/BluePrints/Core-Gameplay/Dodgeballs/DodgeBall Object Reference"))
  (if (`/Game/BluePrints/Core-Gameplay/Dodgeballs/DodgeBall.StarterBall` BallDestroy)
    (`self.K2_DestroyActor` BallDestroy)
    (`/Engine/EditorBlueprintResources/StandardMacros.DecrementInt` (`self.BallCount`)
      (:`  `
        (`KismetSystemLibrary.PrintString` "BallDestroyed")))
    (else
      (`self.K2_DestroyActor` BallDestroy))))

(fn `GetBallSpawns`
  (bind _outactors (`GameplayStatics.GetAllActorsOfClass` "/Game/BluePrints/Core-Gameplay/Ballspawn.Ballspawn_C"))
  (for _array_element _outactors
    (if (`/Game/BluePrints/Core-Gameplay/Ballspawn.isActive` _array_element)
      (`KismetArrayLibrary.Array_AddUnique` (`self.BallSpawns`) _array_element)))
  (`KismetSystemLibrary.PrintString` "Ball Spawns" false))

(fn `SpawnABall`
  (params (BallType :type "/Game/BluePrints/Core-Gameplay/Dodgeballs/DodgeBall Class Reference"))
  (bind _ballspawns (`self.BallSpawns`))
  (`|SpawnActorFromClass` BallType (`self.GetTransform` (`KismetArrayLibrary.Array_Get` _ballspawns (`KismetMathLibrary.RandomInteger` (- (`KismetArrayLibrary.Array_Length` _ballspawns) 1)))) "Undefined" "OverrideRootScale")
  (`/Engine/EditorBlueprintResources/StandardMacros.IncrementInt` (`self.BallCount`)))

(fn `SpawnBalls`
  (bind _asrebound_game_mode (cast `/Game/BluePrints/Gamemodes/ReboundGameMode` (`GameplayStatics.GetGameMode`)))
  (for _array_element (`self.BallSpawns`)
    (`|SpawnActorFromClass` (`/Game/BluePrints/Gamemodes/ReboundGameMode.MainDodgeBall` _asrebound_game_mode) (`self.GetTransform` _array_element) "Undefined" "OverrideRootScale")
    (`/Engine/EditorBlueprintResources/StandardMacros.IncrementInt` (`self.BallCount`)))
  (`KismetSystemLibrary.PrintString` "BallsSpawned"))

(fn `UserConstructionScript`)