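; FractureData records every destructible actor in the level so the breakables can be restored at round start.
; At BeginPlay it binds to the ReboundGameMode start-round event and caches each DestructibleActor's class and transform in parallel arrays, plus WallStats for Fracture_MovingMesh walls.
; On round start it destroys all destructibles, respawns them from the cache, then reapplies moving-wall stats and calls StatsAssigned.
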(event `self.ReceiveBeginPlay`
  (bind _asrebound_game_mode (cast `/Game/BluePrints/Gamemodes/ReboundGameMode` (`GameplayStatics.GetGameMode`)))
  (add `/Game/BluePrints/Gamemodes/ReboundGameMode.startRound` _asrebound_game_mode (delegate `start Round`))
  (`self.getFractureTransforms`)
  (`KismetSystemLibrary.PrintString` (`KismetStringLibrary.TimeSecondsToString` (`KismetSystemLibrary.GetGameTimeInSeconds`))))

(event `start Round`
  (`KismetSystemLibrary.PrintString` "bind working" true true (struct :`R` 1.0 :`G` 0.296274 :`A` 1.0))
  (`self.resetFractures`))

(fn `getFractureTransforms`
  (bind _fracturetrans (`self.fractureTrans`))
  (bind _outactors (`GameplayStatics.GetAllActorsOfClass` "/Script/Engine.DestructibleActor"))
  (for _array_element _outactors
    (`KismetArrayLibrary.Array_Add` (`self.fractureMesh`) (`GameplayStatics.GetObjectClass` _array_element))
    (bind _returnvalue (`KismetArrayLibrary.Array_Add` _fracturetrans (`self.GetTransform` _array_element)))
    (bind _asfracture_moving_mesh (cast `/Game/BluePrints/enviroment/Fracture_MovingMesh` _array_element))
    (`KismetSystemLibrary.PrintString` "moving wall" true true (struct :`R` 0.10593 :`G` 1.0 :`B` 0.065227 :`A` 1.0))
    (`KismetArrayLibrary.Array_Set` (`self.fractureStats`) _returnvalue (`/Game/BluePrints/enviroment/Fracture_MovingMesh.WallStats` _asfracture_moving_mesh) true))
  (`KismetSystemLibrary.PrintString` (`KismetStringLibrary.BuildString_Int` "" "total fractures " (`KismetArrayLibrary.Array_Length` _fracturetrans) "  ") true true (struct :`R` 0.166948 :`G` 1.0 :`A` 1.0)))

(fn `resetFractures`
  (bind _outactors (`GameplayStatics.GetAllActorsOfClass` "/Script/Engine.DestructibleActor"))
  (for _array_element _outactors
    (`self.K2_DestroyActor` _array_element))
  (for (_array_element_2 _array_index) (`self.fractureMesh`)
    (bind _returnvalue (`|SpawnActorFromClass` _array_element_2 (`KismetArrayLibrary.Array_Get` (`self.fractureTrans`) _array_index) "Undefined" "OverrideRootScale"))
    (bind _asfracture_moving_mesh (cast `/Game/BluePrints/enviroment/Fracture_MovingMesh` _returnvalue))
    (set `/Game/BluePrints/enviroment/Fracture_MovingMesh.WallStats` (`KismetArrayLibrary.Array_Get` (`self.fractureStats`) _array_index) _asfracture_moving_mesh)
    (`/Game/BluePrints/enviroment/Fracture_MovingMesh.statsAssigned` _asfracture_moving_mesh))
  (`KismetSystemLibrary.PrintString` (`KismetStringLibrary.BuildString_Int` "" "spawned " _array_index "actors")))

(fn `UserConstructionScript`)