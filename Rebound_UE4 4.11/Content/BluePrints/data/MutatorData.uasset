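; MutatorData is an actor-style Blueprint that spawns a gameplay mutator on BeginPlay and records it in ActiveMutators.
; If the PersisData GameInstance has LoadData set, it spawns the first class in that instance's MutatorsList, otherwise the first in its own TestMutators.
; Only one mutator spawns, at the world origin, and nothing spawns if the GameInstance cast fails.
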(event `self.ReceiveBeginPlay`
  ;[1 1 1] bind events
  (`self.SpawnMutators`))

(fn `SpawnMutators`
  (bind _returnvalue (`KismetMathLibrary.MakeTransform` (0.0 0.0 0.0)))
  (bind _activemutators (`self.activeMutators`))
  (bind _aspersis_data (cast `/Game/BluePrints/data/PersisData` (`GameplayStatics.GetGameInstance`)))
  (if (`/Game/BluePrints/data/PersisData.loadData` _aspersis_data)
    (bind _returnvalue_2 (`|SpawnActorFromClass` (`KismetArrayLibrary.Array_Get` (`/Game/BluePrints/data/PersisData.MutatorsList` _aspersis_data)) _returnvalue "Undefined" "OverrideRootScale"))
    (`KismetArrayLibrary.Array_Add` _activemutators _returnvalue_2)
    (else
      (bind _returnvalue_3 (`|SpawnActorFromClass` (`KismetArrayLibrary.Array_Get` (`self.testMutators`)) _returnvalue "Undefined" "OverrideRootScale"))
      (`KismetArrayLibrary.Array_Add` _activemutators _returnvalue_3))))

(fn `UserConstructionScript`)