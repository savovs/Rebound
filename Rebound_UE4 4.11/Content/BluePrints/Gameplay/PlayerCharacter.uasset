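; Player character for a dodgeball game, which moves by camera-relative capsule impulses and rotates toward the aim axes, shown as a debug line.
; Holding PickUp grabs a nearby DodgeBall through a sphere overlap and Tick pins it to BallSocket; releasing throws it along the aim direction.
; A throw makes the ball ignore its thrower, but the timer subtracts itself, so that immunity ends on the next timer update.
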(event `self.ReceiveBeginPlay`
  (`Controller.Possess` (`GameplayStatics.GetPlayerController` 0) self)
  (bind _asmain_gamemode (cast `/Game/BluePrints/MainGamemode` (`GameplayStatics.GetGameMode`)))
  (`/Game/BluePrints/MainGamemode.AddPC` _asmain_gamemode self))

(event `InputAxis|Vertical`
  (params (AxisValue :type "Float (single-precision)"))
  ;[1 1 1] characterBlend test
  (bind _aschar_test_bp (cast `/Game/Art/charAnimTest/CharTestBP` (`SkeletalMeshComponent.GetAnimInstance` (`self.main_Character`))))
  (`/Game/Art/charAnimTest/CharTestBP.SetVertAxis` _aschar_test_bp AxisValue)
  (bind (_x _y) (`/Game/BluePrints/MainGamemode.GetCameraDir` (stale `self.ReceiveBeginPlay` _asmain_gamemode)))
  (`PrimitiveComponent.AddImpulse` (`self.CapsuleComponent`) (* (* _y (`self.RunningVelocity`)) AxisValue) "None" true))

(event `InputAxis|Horizontal`
  (params (AxisValue :type "Float (single-precision)"))
  (bind _x (`/Game/BluePrints/MainGamemode.GetCameraDir` (stale `self.ReceiveBeginPlay` _asmain_gamemode)))
  (`PrimitiveComponent.AddImpulse` (`self.CapsuleComponent`) (* (* _x (`self.RunningVelocity`)) AxisValue) "None" true))

(event `InputAction|PickUp`
  (params (Key :type "Key Structure" :default "AnyKey"))
  (:`Pressed`
    (bind (_outactors _returnvalue) (`KismetSystemLibrary.SphereOverlapActors_NEW` (`self.K2_GetActorLocation`) (`self.OverlapCircle`) (`|MakeArray` "ObjectTypeQuery2" :!type "EObjectTypeQuery Enum") "/Game/BluePrints/Gameplay/DodgeBall.DodgeBall_C"))
    (if _returnvalue
      (bind _asdodge_ball (cast `/Game/BluePrints/Gameplay/DodgeBall` (`KismetArrayLibrary.Array_Get` _outactors)))
      (`self.PickUpDBall` _asdodge_ball)))
  (:`Released`
    (`self.ThrowDodgeBall` (`self.ThrowVelocity`))))

(event `self.ReceiveTick`
  (params (DeltaSeconds :type "Float (single-precision)"))
  (bind _dodgeball (`self.DodgeBall`))
  (bind _sphere (`/Game/BluePrints/Gameplay/DodgeBall.Sphere` _dodgeball))
  (`self.SetActorRotation` (`KismetMathLibrary.FindLookAtRotation` (`self.K2_GetActorLocation`) (+ (`self.K2_GetActorLocation`) (`KismetMathLibrary.MakeVector` (* (`self.GetInputAxisValue`) 500.0) (* (`self.GetInputAxisValue`) 500.0)))))
  (`self.SelfBallInvincibility`)
  (`self.AimArrowDraw`)
  (if (not (== (`self.DodgeBall`) null))
    (if (`self.IsCarryingDodgeball`)
      (`PrimitiveComponent.SetEnableGravity` _sphere false)
      (`self.K2_SetActorTransform` _dodgeball (`SceneComponent.K2_GetComponentToWorld` (`self.BallSocket`)) false false)
      (`PrimitiveComponent.SetPhysicsLinearVelocity` _sphere (0.0 0.0 0.0) false "None")
      (`PrimitiveComponent.SetPhysicsAngularVelocity` (`/Game/BluePrints/Gameplay/DodgeBall.Sphere` _dodgeball) (0.0 0.0 0.0) false "None")
      (else
        (`PrimitiveComponent.SetEnableGravity` _sphere true)))))

(fn `AimArrowDraw`
  (bind _returnvalue (`self.K2_GetActorLocation`))
  (`KismetSystemLibrary.DrawDebugLine` _returnvalue (+ _returnvalue (`KismetMathLibrary.MakeVector` (* (`self.GetInputAxisValue`) 500.0) (* (`self.GetInputAxisValue`) 500.0))) (struct :`R` 1.0 :`B` 0.188498 :`A` 0.294) 0.0 30.0))

(fn `PickUpDBall`
  (params (DBall :type "/Game/BluePrints/Gameplay/DodgeBall Object Reference"))
  (set `self.DodgeBall` DBall)
  (set `self.IsCarryingDodgeball` true))

(fn `SelfBallInvincibility`
  (bind _dodgeball (`self.DodgeBall`))
  (if (>= (`self.InvincibleSelfTimer`) 0.0)
    (bind _output_get (set `self.InvincibleSelfTimer` (- (`self.InvincibleSelfTimer`) (`self.InvincibleSelfTimer`))))
    (if (and (<= _output_get 0.0) (not (== _dodgeball null)))
      (`PrimitiveComponent.IgnoreActorWhenMoving` (`/Game/BluePrints/Gameplay/DodgeBall.Sphere` _dodgeball) self false))))

(fn `ThrowDodgeBall`
  (params (ThrowVelocity :type "Float (double-precision)"))
  (bind _asmain_gamemode (cast `/Game/BluePrints/MainGamemode` (`GameplayStatics.GetGameMode`)))
  (`/Game/BluePrints/MainGamemode.GetCameraDir` _asmain_gamemode)
  (bind _output_get (set `self.AimDir` (`KismetMathLibrary.MakeVector` (`self.GetInputAxisValue`) (`self.GetInputAxisValue`))))
  (if (`self.IsCarryingDodgeball`)
    (set `self.IsCarryingDodgeball` false)
    (if (not (== _output_get (0.0 0.0 0.0)))
      (bind _returnvalue (* _output_get ThrowVelocity))
      (`PrimitiveComponent.AddImpulse` (`/Game/BluePrints/Gameplay/DodgeBall.Sphere` (`self.DodgeBall`)) _returnvalue "None" true)
      (`KismetSystemLibrary.PrintString` (`KismetStringLibrary.Conv_VectorToString` _returnvalue))
      (`PrimitiveComponent.IgnoreActorWhenMoving` (`/Game/BluePrints/Gameplay/DodgeBall.Sphere` (`self.DodgeBall`)) self true)
      (set `self.InvincibleSelfTimer` 2.0))))

(fn `UserConstructionScript`)