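; Main menu game mode for Rebound that runs a local lobby for up to four gamepad players.
; BeginPlay shows the menu widget and creates local players, then Tick polls face buttons to join, leave or toggle ready, notifying through Call events.
; PlayerOrder maps menu slots to controllers, refilling freed slots.
; When all active players are ready, StartGame saves the order to the PersistentData game instance and opens MainMenuBP's first level.
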(event EventBeginPlay
  (bind _returnvalue (UserInterface|CreateWidget "/Game/UI/MainMenu/MainMenuUI.MainMenuUI_C"))
  (UserInterface|Viewport|AddtoViewport _returnvalue 0)
  (CallFunction|CreatePlayers)
  ;[1 1 1] show mouse
  (Variables|/Script/Engine.PlayerController|SetbShowMouseCursor (Game|GetPlayerController 0) true))

(event EventTick
  (params (DeltaSeconds :type Float%20%28single-precision%29))
  (CallFunction|CheckforNewPlayers)
  (CallFunction|CheckforRemovePlayer)
  (CallFunction|CheckforReady))

(fn ConstructionScript)

(fn CreatePlayers
  (for _index (range 0 3)
    (Class|GameplayStatics|CreatePlayer -1)))

(fn CheckforNewPlayers
  (bind _playerorder (Variables|Default|GetPlayerOrder))
  (for _index (range 0 3)
    (if (and (Game|Player|WasInputKeyJustPressed (Game|GetPlayerController _index) "Gamepad_FaceButton_Bottom") (not (Utilities|Array|Get(acopy) (Variables|Default|GetplayerActiveArray) _index)))
      (Utilities|Array|SetArrayElem _playerorder (Variables|Default|GetcurPlayerID) _index)
      (bind (_array_element _array_index) (Utilities|Array|ForEachLoopwithBreak _playerorder :!label _label)
        (:LoopBody
          (if (== _array_element -1)
            (Variables|Default|SetcurPlayerID _array_index)
            (goto _label Break)))
        (:Completed
          (Utilities|Array|SetArrayElem (Variables|Default|GetplayerActiveArray) _index true)
          (Default|CallPlayerAdded _index)
          (Development|PrintString (Utilities|String|BuildString(Integer) "" "player" _index "added")))))))

(fn CheckforRemovePlayer
  (bind _playerorder (Variables|Default|GetPlayerOrder))
  (for _index (range 0 3)
    (if (and (Game|Player|WasInputKeyJustPressed (Game|GetPlayerController _index) "Gamepad_FaceButton_Right") (Utilities|Array|Get(acopy) (Variables|Default|GetplayerActiveArray) _index))
      (Default|CallPlayerRemoved (Utilities|Array|FindItem _playerorder _index))
      (Variables|Default|SetcurPlayerID (Utilities|Array|FindItem _playerorder _index))
      (Utilities|Array|SetArrayElem _playerorder (Utilities|Array|FindItem _playerorder _index) -1)
      (Utilities|Array|SetArrayElem (Variables|Default|GetplayerActiveArray) _index false)
      (Utilities|Array|SetArrayElem (Variables|Default|GetplayerReadyArray) _index false)
      (Default|CallPlayerReady (Variables|Default|GetcurPlayerID) false)
      (Development|PrintString (Utilities|String|BuildString(Integer) "" "player" _index "removed")))))

(fn StartGame
  (bind _playerorder (Variables|Default|GetPlayerOrder))
  (bind _aspersistent_data (Utilities|Casting|CastToPersistentData (Game|GetGameInstance)))
  (Variables|/Game/BluePrints/data/PersistentData.PersistentData_C|SetloadData _aspersistent_data true)
  (Variables|/Game/BluePrints/data/PersistentData.PersistentData_C|SetPlayers _aspersistent_data _playerorder)
  (for (_array_element _array_index) _playerorder
    (Development|PrintString (Utilities|String|BuildString(Integer) (Utilities|String|BuildString(Integer) "" "player pos" _array_index "contains ") "player ID" _array_element)))
  (Default|CallAllPlayersReady)
  ;[1 1 1] load level
  (bind _outactors (Actor|GetAllActorsOfClass "/Game/UI/MainMenu/MainMenuBP.MainMenuBP_C"))
  (Game|OpenLevel(byName) (Utilities|Array|Get(acopy) (Variables|/Game/UI/MainMenu/MainMenuBP.MainMenuBP_C|Getlevels (Utilities|Array|Get(acopy) _outactors)))))

(fn CheckforReady
  (bind _playerreadyarray (Variables|Default|GetplayerReadyArray))
  (for _index (range 0 3)
    (if (and (Game|Player|WasInputKeyJustPressed (Game|GetPlayerController _index) "Gamepad_FaceButton_Top") (Utilities|Array|Get(acopy) (Variables|Default|GetplayerActiveArray) _index))
      (Default|CallPlayerReady (Utilities|Array|FindItem (Variables|Default|GetPlayerOrder) _index) (not (Utilities|Array|Get(acopy) _playerreadyarray _index)))
      (Utilities|Array|SetArrayElem _playerreadyarray _index (not (Utilities|Array|Get(acopy) _playerreadyarray _index)))))
  (bind (_array_element _array_index) (Utilities|Array|ForEachLoopwithBreak (Variables|Default|GetplayerActiveArray) :!label _label)
    (:LoopBody
      (if _array_element
        (if (Utilities|Array|Get(acopy) (Variables|Default|GetplayerReadyArray) _array_index)
          (LocalVariables|Setplay true)
          (else
            (LocalVariables|Setplay false)
            (goto _label Break)))))
    (:Completed
      (if (LocalVariables|Getplay)
        (CallFunction|StartGame)))))