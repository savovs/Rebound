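; Main game mode that spawns the player characters, keeps the list of them and creates the game UI.
; SpawnPlayers places one character per index at the matching spawn point, assigns its PlayerID, then builds a GameUI widget set up for the player count.
; AddPC registers a character without duplicates, and GetCameraDir returns the first player camera's world-space right and up vectors.
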(fn `AddPC`
  (params (playerCharacter :type "/Game/BluePrints/Core-Gameplay/PlayerCharacter Object Reference"))
  (`KismetArrayLibrary.Array_AddUnique` (`self.Players`) playerCharacter))

(fn `GetCameraDir`
  (returns (X :type "Vector Structure") (Y :type "Vector Structure"))
  (bind _returnvalue (`self.GetTransform` (`GameplayStatics.GetPlayerCameraManager` 0)))
  (return (`KismetMathLibrary.TransformDirection` _returnvalue (0.0 1.0 0.0)) (`KismetMathLibrary.TransformDirection` _returnvalue (0.0 0.0 1.0))))

(fn `SpawnPlayers`
  (params (playerCount :type Integer) (spawnPoints :type "Array of Actor Object Reference"))
  (set `self.SpawnPoints` spawnPoints)
  (for _index (range (+ playerCount 1))
    (bind _returnvalue (`|SpawnActorFromClass` "/Game/BluePrints/Core-Gameplay/PlayerCharacter.PlayerCharacter_C" (`self.GetTransform` (`KismetArrayLibrary.Array_Get` (`self.SpawnPoints`) _index)) "Undefined" "OverrideRootScale"))
    (set `/Game/BluePrints/Core-Gameplay/PlayerCharacter.PlayerID` _index _returnvalue)
    (`KismetArrayLibrary.Array_Add` (`self.Players`) _returnvalue))
  (bind _returnvalue_2 (`|CreateWidget` "/Game/UI/GameUI_test/GameUI.GameUI_C"))
  (`/Game/UI/GameUI_test/GameUI.SetupUI` _returnvalue_2 playerCount)
  (`UserWidget.AddToViewport` _returnvalue_2 0))

(fn `UserConstructionScript`)