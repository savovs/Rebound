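; Game mode for Rebound, a local multiplayer dodgeball game that runs rounds and keeps per-player scores.
; Setup finds or spawns GameData, creates controllers from it or saved PersisData, adds UI and runs pre-game mutators.
; Each round respawns pawns and spawns balls at active spawn points.
; Dodgeball kills adjust scores, penalising self-hits; destroyed starter balls respawn, and a new round starts when the player counter runs out.
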(event `self.ReceiveBeginPlay`
  (`self.GameSetup`))

(fn `createBalls`
  (params (starterBalls :type Boolean))
  (bind _dodgeball (`self.DodgeBall`))
  (bind _ballspawns (`self.BallSpawns`))
  (if (`/Game/BluePrints/Core-Gameplay/GameData.CreateBallsOnAllSpawns` (`self.gameData`))
    (for _array_element _ballspawns
      (bind _returnvalue (`|SpawnActorFromClass` _dodgeball (`self.GetTransform` _array_element) "Undefined" "OverrideRootScale"))
      (if (not starterBalls)
        (set `/Game/BluePrints/Core-Gameplay/Dodgeballs/DodgeBall.StarterBall` false _returnvalue)))
    (else
      (bind _returnvalue_2 (`|SpawnActorFromClass` _dodgeball (`self.GetTransform` (`KismetArrayLibrary.Array_Get` _ballspawns (`KismetMathLibrary.RandomIntegerInRange` 0 (- (`KismetArrayLibrary.Array_Length` _ballspawns) 1)))) "Undefined" "OverrideRootScale"))
      (if (not starterBalls)
        (set `/Game/BluePrints/Core-Gameplay/Dodgeballs/DodgeBall.StarterBall` false _returnvalue_2)))))

(fn `createPawns`
  (for _index (range (+ (`/Game/BluePrints/Core-Gameplay/GameData.playerCount` (`self.gameData`)) 1))
    (bind _returnvalue (`GameplayStatics.GetPlayerController` _index))
    (bind _asrebound_player_controller (cast `/Game/BluePrints/Core-Gameplay/ReboundPlayerController` _returnvalue))
    (`/Game/BluePrints/Core-Gameplay/ReboundPlayerController.SpawnPawn` _asrebound_player_controller (`self.GetTransform` (`self.K2_FindPlayerStart` _returnvalue)) (`self.PlayerPawn`)))
  (bind _outactors (`GameplayStatics.GetAllActorsOfClass` "/Game/BluePrints/Core-Gameplay/ReboundPlayerCharacter.ReboundPlayerCharacter_C"))
  (set `self.Players` _outactors))

(fn `CreatePlayers`
  (params (PlayerCount :type Integer))
  (for _index (range 1 (+ PlayerCount 1))
    (bind _returnvalue (`GameplayStatics.CreatePlayer` _index))
    (bind _asrebound_player_controller (cast `/Game/BluePrints/Core-Gameplay/ReboundPlayerController` _returnvalue))
    (bind _output_get (set `/Game/BluePrints/Core-Gameplay/ReboundPlayerController.PlayerID` _index _asrebound_player_controller))
    (`KismetSystemLibrary.PrintString` (`KismetStringLibrary.Concat_StrStr` (`KismetStringLibrary.Conv_IntToString` _output_get) "Player created") false)))

(fn `DestroyBall`
  (params (Ball :type "/Game/BluePrints/Core-Gameplay/Dodgeballs/DodgeBall Object Reference"))
  (bind _ballspawns (`self.BallSpawns`))
  (if (not (`self.IsActorBeingDestroyed` Ball))
    (`KismetArrayLibrary.Array_RemoveItem` (`self.Balls`) Ball)
    (if (`/Game/BluePrints/Core-Gameplay/Dodgeballs/DodgeBall.StarterBall` Ball)
      (`self.K2_DestroyActor` Ball)
      (`|SpawnActorFromClass` (`self.DodgeBall`) (`self.GetTransform` (`KismetArrayLibrary.Array_Get` _ballspawns (`KismetMathLibrary.RandomInteger` (- (`KismetArrayLibrary.Array_Length` _ballspawns) 1)))) "Undefined" "OverrideRootScale")
      (else
        (`self.K2_DestroyActor` Ball)))))

(fn `GameSetup`
  (`self.SpawnGameData`)
  (`self.SetUpBallSpawns`)
  (`KismetSystemLibrary.PrintString` "new game")
  ;[1 1 1] add UI
  (bind _returnvalue (`|CreateWidget` "/Game/UI/GameUI_test/GameUI.GameUI_C"))
  (`UserWidget.AddToViewport` _returnvalue 0)
  (bind _aspersis_data (cast `/Game/BluePrints/Core-Gameplay/PersisData` (`GameplayStatics.GetGameInstance`)))
  (if (`/Game/BluePrints/Core-Gameplay/PersisData.loadData` _aspersis_data)
    (bind _players (`/Game/BluePrints/Core-Gameplay/PersisData.Players` _aspersis_data))
    ;[1 1 1] create the controllers from the persisData
    (`self.CreatePlayers` _players)
    (set `/Game/BluePrints/Core-Gameplay/GameData.playerCount` _players (`self.gameData`))
    (else
      ;[1 1 1] create the controllers from the gamedata
      (`self.CreatePlayers` (`/Game/BluePrints/Core-Gameplay/GameData.playerCount` (`self.gameData`)))))
  (`self.StartGame`)
  ;[1 1 1] call pre game mutators (replace with the event callers)
  (for _array_element (`/Game/BluePrints/Core-Gameplay/GameData.ActiveMutators` (`self.gameData`))
    (`/Game/BluePrints/Core-Gameplay/mutators/Mutator.preGame` _array_element))
  (`self.StartGame`)
  (`self.RoundSetup`))

(fn `playerDied`
  (params (BallID :type Integer) (HitID :type Integer) (KilledByDodgeball :type Boolean) (player :type "/Game/BluePrints/Core-Gameplay/ReboundPlayerCharacter Object Reference"))
  (bind _scores (`self.Scores`))
  (bind _item (`KismetArrayLibrary.Array_Get` _scores BallID))
  (if (not (`self.IsActorBeingDestroyed` player))
    (`KismetArrayLibrary.Array_RemoveItem` (`self.Players`) player)
    (`/Game/BluePrints/Core-Gameplay/ReboundPlayerCharacter.DropBall` player)
    (`self.K2_DestroyActor` player)
    (if KilledByDodgeball
      (if (== BallID HitID)
        (`KismetArrayLibrary.Array_Set` _scores BallID (- _item 1))
        (else
          (`KismetArrayLibrary.Array_Set` _scores BallID (+ _item 1)))))
    (bind _result (`/Engine/EditorBlueprintResources/StandardMacros.DecrementInt` (`self.currentPlayers`))
      (:`  `
        (if (<= _result 0)
          (`self.RoundSetup`))))))

(fn `RoundSetup`
  (bind _players (`self.Players`))
  (bind _balls (`self.Balls`))
  (`KismetSystemLibrary.PrintString` "new round")
  (`/Engine/EditorBlueprintResources/StandardMacros.IncrementInt` (`self.round`)
    (:`  `
      ;[1 1 1] destroy the old players in the scene
      (for _array_element _players
        (`self.K2_DestroyActor` _array_element))
      (`KismetArrayLibrary.Array_Clear` _players)
      ;[1 1 1] destroy the old balls in the scene
      (for _array_element_2 _balls
        (if (!= _array_element_2 null)
          (`self.K2_DestroyActor` _array_element_2)))
      (`KismetArrayLibrary.Array_Clear` _balls)
      (set `self.currentPlayers` (`/Game/BluePrints/Core-Gameplay/GameData.playerCount` (`self.gameData`)))
      (`self.createPawns`)
      (`self.createBalls` true)
      (`self.startRound`))))

(fn `SetUpBallSpawns`
  (bind _outactors (`GameplayStatics.GetAllActorsOfClass` "/Game/BluePrints/Core-Gameplay/Ballspawn.Ballspawn_C"))
  (for _array_element _outactors
    (if (`/Game/BluePrints/Core-Gameplay/Ballspawn.isActive` _array_element)
      (`KismetArrayLibrary.Array_AddUnique` (`self.BallSpawns`) _array_element)))
  (`KismetSystemLibrary.PrintString` "Ball Spawns" false))

(fn `SpawnGameData`
  (bind _outactors (`GameplayStatics.GetAllActorsOfClass` "/Game/BluePrints/Core-Gameplay/GameData.GameData_C"))
  (if (< (`KismetArrayLibrary.Array_Length` _outactors) 1)
    (bind _returnvalue (`|SpawnActorFromClass` "/Game/BluePrints/Core-Gameplay/GameData.GameData_C" (`KismetMathLibrary.MakeTransform` (0.0 0.0 0.0)) "Undefined" "OverrideRootScale"))
    (set `self.gameData` _returnvalue)
    (else
      (set `self.gameData` (`KismetArrayLibrary.Array_Get` _outactors)))))

(fn `UserConstructionScript`)