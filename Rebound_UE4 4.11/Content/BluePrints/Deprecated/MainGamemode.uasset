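; Dodgeball game mode, filed under Deprecated, that runs rounds, scoring and ball spawning.
; SetupGame stores GameData, starts a round, then calls PreGame on active mutators.
; ChangeScore rewards the ball's owner or penalizes self-hits, starting a new round when the player count reaches zero.
; NewRound clears actors and spawns a ball, but SpawnPlayers is empty, its character and UI creation logic left disconnected.
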(fn `AddPC`
  (params (playerCharacter :type "/Game/BluePrints/Deprecated/PlayerCharacter Object Reference"))
  (`KismetArrayLibrary.Array_AddUnique` (`self.Players`) playerCharacter))

(fn `changeScore`
  (params (ballID :type Integer) (hitID :type Integer))
  (bind _scores (`self.Scores`))
  (bind _item (`KismetArrayLibrary.Array_Get` _scores ballID))
  (if (== ballID hitID)
    (`KismetArrayLibrary.Array_Set` _scores ballID (- _item 1))
    (else
      (`KismetArrayLibrary.Array_Set` _scores ballID (+ _item 1))))
  (bind _result (`/Engine/EditorBlueprintResources/StandardMacros.DecrementInt` (`self.currentPlayers`))
    (:`  `
      (if (== _result 0)
        (`self.newRound`)))))

(fn `GetCameraDir`
  (returns (X :type "Vector Structure") (Y :type "Vector Structure"))
  (bind _returnvalue (`self.GetTransform` (`GameplayStatics.GetPlayerCameraManager` 0)))
  (return (`KismetMathLibrary.TransformDirection` _returnvalue (0.0 1.0 0.0)) (`KismetMathLibrary.TransformDirection` _returnvalue (0.0 0.0 1.0))))

(fn `newRound`
  (bind _players (`self.Players`))
  (bind _balls (`self.Balls`))
  (`/Engine/EditorBlueprintResources/StandardMacros.IncrementInt` (`self.round`)
    (:`  `
      (for _array_element _players
        (`self.K2_DestroyActor` _array_element))
      (`KismetArrayLibrary.Array_Clear` _players)
      (for _array_element_2 _balls
        (`self.K2_DestroyActor` _array_element_2))
      (`KismetArrayLibrary.Array_Clear` _balls)
      (set `self.currentPlayers` (`/Game/BluePrints/Core-Gameplay/GameData.playerCount` (`self.gameData`)))
      (`self.SpawnPlayers`)
      (`self.SpawnBall`))))

(fn `setupGame`
  (params (gameData :type "/Game/BluePrints/Core-Gameplay/GameData Object Reference"))
  (set `self.gameData` gameData)
  (`self.newRound`)
  (for _array_element (`/Game/BluePrints/Core-Gameplay/GameData.ActiveMutators` (`self.gameData`))
    (`/Game/BluePrints/Core-Gameplay/mutators/Mutator.preGame` _array_element)))

(fn `SpawnBall`
  (bind _balls (`self.Balls`))
  (bind _returnvalue (`|SpawnActorFromClass` "/Game/BluePrints/Core-Gameplay/Dodgeballs/DodgeBall.DodgeBall_C" (`KismetMathLibrary.MakeTransform` (0.0 0.0 0.0)) "Undefined" "OverrideRootScale"))
  (`KismetArrayLibrary.Array_Resize` _balls (+ (`KismetArrayLibrary.Array_Length` _balls) 1))
  (`KismetArrayLibrary.Array_Add` _balls _returnvalue))

(fn `SpawnPlayers`)

(fn `UserConstructionScript`)