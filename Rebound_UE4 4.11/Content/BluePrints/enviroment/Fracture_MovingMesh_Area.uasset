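; Fracture_MovingMesh_Area is a trigger area Blueprint that toggles a wall when a DodgeBall leaves its sphere.
; The construction script scales SphereTrigger from the TriggerSize field of WallStats.
; On end overlap, a cast to DodgeBall gates a call to ToggleWall, followed by a debug print.
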(event `self.SphereTrigger.OnComponentEndOverlap`
  (params (OtherActor :type "Actor Object Reference") (OtherComp :type "PrimitiveComponent Object Reference") (OtherBodyIndex :type Integer))
  (cast `/Game/BluePrints/Core-Gameplay/Dodgeballs/DodgeBall` OtherActor)
  (`self.toggleWall`)
  (`KismetSystemLibrary.PrintString` "toggleWAll"))

(fn `UserConstructionScript`
  (`parent.UserConstructionScript`)
  (`SceneComponent.SetWorldScale3D` (`self.SphereTrigger`) (`.triggerSize_21_60C4069A4D71D889FD5143B21DA9387D` (break `/Game/BluePrints/enviroment/WallStats` (`self.WallStats`)))))