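; A wall mesh actor that slides vertically between up and down heights when toggled by the first FractureData actor or any WallPressurePlate.
; Once wall stats are assigned it caches travel distance, binds those toggle events and toggles once if configured to start down.
; Each toggle flips the target and disables collision; Tick then lerps Z by elapsed time and speed, restoring collision on arrival.
; Debug strings print throughout.
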(event `self.ReceiveBeginPlay`)

(event `statsAssigned`
  (bind (_startingposup _uppoint _downpoint) (break `/Game/BluePrints/enviroment/WallStats` (`self.WallStats`)))
  (set `self.distance` (`KismetMathLibrary.VSize` (- _uppoint _downpoint)))
  (set `self.CurPosUp` (`.startingPosUp_22_670EC4264E748D4054EEA5AD0851CEFF` (break `/Game/BluePrints/enviroment/WallStats` (`self.WallStats`))))
  (bind _outactors (`GameplayStatics.GetAllActorsOfClass` "/Game/BluePrints/data/FractureData.FractureData_C"))
  (add `/Game/BluePrints/data/FractureData.ToggleWall` (`KismetArrayLibrary.Array_Get` _outactors) (delegate `Toggle wall`))
  (bind _outactors_2 (`GameplayStatics.GetAllActorsOfClass` "/Game/BluePrints/enviroment/wallPressurePlate.wallPressurePlate_C"))
  (for _array_element _outactors_2
    (add `/Game/BluePrints/enviroment/wallPressurePlate.ToggleWall` _array_element (delegate `Toggle wall`))
    (`KismetSystemLibrary.PrintString` (`KismetSystemLibrary.GetDisplayName` _array_element) true true (struct :`R` 1.0 :`G` 0.431561 :`A` 1.0) 10.0))
  (if (not (`self.CurPosUp`))
    (`self.toggleWall`)
    (`KismetSystemLibrary.PrintString` "DEFAULT DOWN" true true (struct :`R` 1.0 :`G` 0.517984 :`A` 1.0))))

(event `Toggle wall`
  (`self.toggleWall`)
  (`KismetSystemLibrary.PrintString` "toggle" true true (struct :`R` 1.0 :`G` 0.653048 :`B` 0.1 :`A` 1.0))
  (if (`self.moveWall`) :!label _label
    (`self.moveWallUp`)))

(event `self.ReceiveTick`
  (params (DeltaSeconds :type "Float (single-precision)"))
  (`parent.ReceiveTick` DeltaSeconds)
  (goto _label))

(fn `moveWallUp`
  (bind (_startingposup _uppoint _downpoint) (break `/Game/BluePrints/enviroment/WallStats` (`self.WallStats`)))
  (bind _returnvalue (/ (* (- (`KismetSystemLibrary.GetGameTimeInSeconds`) (`self.startTime`)) (`.speed_13_54EFAF264617A3264C0454B2313CF6D3` (break `/Game/BluePrints/enviroment/WallStats` (`self.WallStats`)))) (`self.distance`)))
  (`self.K2_SetActorTransform` (`KismetMathLibrary.TLerp` (`self.starting point`) (`KismetMathLibrary.MakeTransform` (`KismetMathLibrary.MakeVector` (.x (.location (`self.GetTransform`))) (.y (.location (`self.GetTransform`))) (.z (`KismetMathLibrary.SelectVector` _uppoint _downpoint (`self.CurPosUp`)))) (.rotation (`self.GetTransform`)) (.scale (`self.GetTransform`))) _returnvalue))
  (if (>= _returnvalue 1.0)
    (set `self.moveWall` false)
    (`self.SetActorEnableCollision` true)
    (`KismetSystemLibrary.PrintString` "stop wall")
    (else
      (`KismetSystemLibrary.PrintString` (`KismetStringLibrary.Conv_DoubleToString` _returnvalue)))))

(fn `toggleWall`
  (set `self.CurPosUp` (select `bool` (`self.CurPosUp`) :`false` true))
  (set `self.moveWall` true)
  (set `self.starting point` (`self.GetTransform`))
  (set `self.startTime` (`KismetSystemLibrary.GetGameTimeInSeconds`))
  (`self.SetActorEnableCollision` false))

(fn `UserConstructionScript`
  (`parent.UserConstructionScript`))